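; BP_PlayerCharacter is the player-controlled character, handling jump, sideways movement and camera zoom input.
; MoveRight adds movement along the fixed world X axis, so lateral movement does not follow control rotation.
; The Zoom axis feeds a Zoom function that scales the input and adjusts the spring arm length within a clamped range.
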(event Input|ActionEvents|InputActionJump
  (params (Key :type Key%20Structure :default "AnyKey"))
  (:Pressed
    (Character|Jump)))

(event Input|AxisEvents|InputAxisMoveRight
  (params (AxisValue :type Float%20%28single-precision%29))
  (Pawn|Input|AddMovementInput "1.000000, 0, 0" AxisValue false))

(event Input|AxisEvents|InputAxisZoom
  (params (AxisValue :type Float%20%28single-precision%29))
  (CallFunction|Zoom AxisValue))

(fn ConstructionScript)

(fn Zoom
  (params (A :type Float%20%28single-precision%29))
  (bind _springarm (Variables|Default|GetSpringArm))
  (Variables|/Script/Engine.SpringArmComponent|SetTargetArmLength _springarm (Math|Float|Clamp(Float) (+ (* A 2e+01) (Variables|/Script/Engine.SpringArmComponent|GetTargetArmLength _springarm)) 5e+02 1e+03)))